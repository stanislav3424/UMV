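; TestUnit is a test unit Blueprint that exercises the inventory and equipment system when play begins.
; BeginPlay constructs and initializes a MyInventory and puts it on in the Backpack equipment slot via PutOnEquipment.
; It then creates two BP_Item_Test items and adds them at separate inventory indices, storing the second add's result in NewVar0.
; Setup is chained through validity checks, and Tick, overlap and the construction script do nothing.
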(event `self.ReceiveBeginPlay`
  (bind _returnvalue (`|GenericCreateObject` "/Game/Blueprint/MyInventory.MyInventory_C"))
  (`/Engine/EditorBlueprintResources/StandardMacros.IsValid` _returnvalue
    (:`Is Valid`
      (`Inventory.Initialization` _returnvalue)
      (`self.PutOnEquipment` _returnvalue "Backpack")
      (bind _returnvalue_2 (`|GenericCreateObject` "/Game/BP_Item_Test.BP_Item_Test_C"))
      (`/Engine/EditorBlueprintResources/StandardMacros.IsValid` _returnvalue_2
        (:`Is Valid`
          (`Inventory.Initialization` _returnvalue_2)
          (`Inventory.AddToInventory` _returnvalue _returnvalue_2 0)
          (bind _returnvalue_3 (`|GenericCreateObject` "/Game/BP_Item_Test.BP_Item_Test_C"))
          (`/Engine/EditorBlueprintResources/StandardMacros.IsValid` _returnvalue_3
            (:`Is Valid`
              (`Inventory.Initialization` _returnvalue_3)
              (bind _returnvalue_4 (`Inventory.AddToInventory` _returnvalue _returnvalue_3 3))
              (set `self.NewVar_0` _returnvalue_4))))))))

(fn `UserConstructionScript`)